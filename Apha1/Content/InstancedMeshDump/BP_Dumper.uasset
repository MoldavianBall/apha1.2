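; BP_Dumper is a utility actor that copies instanced static meshes out of a running level into save games and can rebuild them.
; Shortly after BeginPlay it scans every actor's InstancedStaticMeshComponents, saving each one's mesh and world-space instance transforms to a SavingData slot named from actor plus component.
; LoadDump reads the slots listed in Slot and spawns a BP_DumpedActor for each to recreate the instances.
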(event Custom|StartDump
  (bind _outactors (Actor|GetAllActorsOfClass "/Script/Engine.Actor"))
  (for _array_element _outactors
    (for _array_element_2 (Actor|GetComponentsByClass _array_element "/Script/Engine.InstancedStaticMeshComponent")
      (Utilities|IsValid _array_element_2
        (:Is%20Valid
          (bind _returnvalue (SaveGame|CreateSaveGameObject "/Game/InstancedMeshDump/SavingData.SavingData_C"))
          (bind _assaving_data (Utilities|Casting|CastToSavingData _returnvalue))
          (for _index (range 0 (- (Components|InstancedStaticMesh|GetInstanceCount _array_element_2) 1))
            (Utilities|Array|Add (Variables|/Game/InstancedMeshDump/SavingData.SavingData_C|GetTransforms _assaving_data) (.OutInstanceTransform (Components|InstancedStaticMesh|GetInstanceTransform _array_element_2 _index true)))
            (Variables|/Game/InstancedMeshDump/SavingData.SavingData_C|SetMesh _assaving_data (Variables|/Script/Engine.StaticMeshComponent|GetStaticMesh _array_element_2)))
          (SaveGame|SaveGametoSlot _returnvalue (Utilities|String|Append (Utilities|GetObjectName _array_element) (Utilities|GetObjectName _array_element_2))))))))

(event Custom|LoadDump
  (for _array_element (Variables|Default|GetSlot)
    (bind _returnvalue (SaveGame|DoesSaveGameExist _array_element))
    (if _returnvalue
      (bind _returnvalue_2 (SaveGame|LoadGamefromSlot _array_element))
      (bind _assaving_data (Utilities|Casting|CastToSavingData _returnvalue_2))
      (bind _returnvalue_3 (Game|SpawnActorfromClass "/Game/InstancedMeshDump/BP_DumpedActor.BP_DumpedActor_C" (Math|Transform|MakeTransform "0, 0, 0" "0, 0, 0" "1,1,1") true 0 0))
      (Components|StaticMesh|SetStaticMesh (Variables|/Game/InstancedMeshDump/BP_DumpedActor.BP_DumpedActor_C|GetInstancedStaticMesh _returnvalue_3) (Variables|/Game/InstancedMeshDump/SavingData.SavingData_C|GetMesh _assaving_data))
      (Variables|/Game/InstancedMeshDump/BP_DumpedActor.BP_DumpedActor_C|SetInstances _returnvalue_3 (Variables|/Game/InstancedMeshDump/SavingData.SavingData_C|GetTransforms _assaving_data))
      (Default|Spawn _returnvalue_3))))

(event EventBeginPlay
  (Utilities|FlowControl|Delay 0.2)
  (CallFunction|StartDump))

(fn ConstructionScript)