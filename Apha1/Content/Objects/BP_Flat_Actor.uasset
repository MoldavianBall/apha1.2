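; BP_Flat_Actor is a physical object that can be picked up, with sounds for pickup and impact.
; BeginPlay assigns the hit and pick sounds to the Drop and Pick audio components.
; PickUp disables physics and collision and plays the pick sound, while Hit re-enables both.
; Static mesh hits play the drop sound after a short delay, and SetSocket is an empty event.
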(event OnComponentHit(StaticMesh)
  (params (HitComponent :type Primitive%20Component%20Object%20Reference) (OtherActor :type Actor%20Object%20Reference) (OtherComp :type Primitive%20Component%20Object%20Reference) (NormalImpulse :type Vector :default "0, 0, 0") (Hit :type Hit%20Result%20Structure%20%28by%20ref%29))
  (Utilities|FlowControl|Delay 0.2)
  (Audio|Components|Audio|Play (Variables|Default|GetDrop) 0.0))

(event Custom|Hit
  (Physics|SetSimulatePhysics (Variables|Default|GetStaticMesh) true)
  (Collision|SetActorEnableCollision true))

(event Custom|Pick%20Up
  (bind _staticmesh (Variables|Default|GetStaticMesh))
  (Physics|SetSimulatePhysics _staticmesh false)
  (Physics|SetSimulatePhysics _staticmesh false)
  (Collision|SetActorEnableCollision false)
  (Audio|Components|Audio|Play (Variables|Default|GetPick) 0.0))

(event Custom|Set%20Socket)

(event EventBeginPlay
  (Audio|Components|Audio|SetSound (Variables|Default|GetDrop) (Variables|Default|GetHit%20Sound))
  (Audio|Components|Audio|SetSound (Variables|Default|GetPick) (Variables|Default|GetPick%20Sound)))

(event Collision|EventActorBeginOverlap
  (params (OtherActor :type Actor%20Object%20Reference)))

(event EventTick
  (params (DeltaSeconds :type Float%20%28single-precision%29)))

(fn ConstructionScript)