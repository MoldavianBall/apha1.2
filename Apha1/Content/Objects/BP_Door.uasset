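; BP_Door is an interactable door that swings its mesh open or shut with sound, or plays a locked sound instead.
; Interact checks that the passed value is the door mesh, then either calls Locked when Loc is set or alternates Open and Close through a FlipFlop.
; Open and Close each run a timed MoveComponentTo rotation and stop the opposing one, allowing reversal mid-swing.
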(event Custom|Close
  ;[1 1 1] Door Events
  (Utilities|FlowControl|Sequence
    (:then_0
      (Audio|PlaySoundatLocation "/Game/Sounds/door_open_Cue.door_open_Cue" (Transformation|GetActorLocation) "0, 0, 0" 1.0 1.0 0.0 0 0 0)
      (Components|MoveComponentTo (Variables|Default|GetStaticMesh1) "0, 0, 0" "0,0.000000, 0" false false 0.4 false))
    (:then_1
      (Components|MoveComponentTo (Variables|Default|GetStaticMesh1) "0, 0, 0" "0,90.000000, 0" false false 0.4 false) ; enters at Stop
    )))

(event Custom|Open
  ;[1 1 1] Door Events
  (Utilities|FlowControl|Sequence
    (:then_0
      (Audio|PlaySoundatLocation "/Game/Sounds/door_open_Cue.door_open_Cue" (Transformation|GetActorLocation) "0, 0, 0" 1.0 1.0 0.0 0 0 0)
      (Components|MoveComponentTo (Variables|Default|GetStaticMesh1) "0, 0, 0" "0,90.000000, 0" false false 0.4 false))
    (:then_1
      (Components|MoveComponentTo (Variables|Default|GetStaticMesh1) "0, 0, 0" "0,0.000000, 0" false false 0.4 false) ; enters at Stop
    )))

(event Custom|Locked
  ;[1 1 1] Door Events
  (Audio|PlaySoundatLocation "/Game/Sounds/door_locked_Cue.door_locked_Cue" (Transformation|GetActorLocation) "0, 0, 0" 1.0 1.0 0.0 0 0 0))

(event EventBeginPlay)

(event Collision|EventActorBeginOverlap
  (params (OtherActor :type Actor%20Object%20Reference)))

(event EventTick
  (params (DeltaSeconds :type Float%20%28single-precision%29)))

(event EventInteract
  (params (NewParam :type Primitive%20Component%20Object%20Reference))
  (if (== NewParam (Variables|Default|GetStaticMesh1))
    (if (Variables|Default|GetLoc?)
      (CallFunction|Locked)
      (else
        (Utilities|FlowControl|FlipFlop
          (:A
            (CallFunction|Open))
          (:B
            (CallFunction|Close)))))))

(fn ConstructionScript)